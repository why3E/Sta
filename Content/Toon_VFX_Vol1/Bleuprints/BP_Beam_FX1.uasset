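; Beam VFX actor from a toon effects pack that replays a two-stage Niagara effect in an endless loop.
; The construction script assigns the System and Beam variables as assets on two Niagara components.
; From BeginPlay it restarts the first component, waits a fixed delay, restarts the beam component, then waits SpawnInterval before repeating.
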(event `self.ReceiveBeginPlay`
  (`ActorComponent.Activate` (`self.Niagara`) true :!label _label)
  (`KismetSystemLibrary.Delay` 4.0)
  (`ActorComponent.Activate` (`self.Niagara1`) true)
  (`KismetSystemLibrary.Delay` (`self.Spawn interval`))
  (goto _label))

(fn `UserConstructionScript`
  (`NiagaraComponent.SetAsset` (`self.Niagara`) (`self.System`))
  (`NiagaraComponent.SetAsset` (`self.Niagara1`) (`self.Beam`)))